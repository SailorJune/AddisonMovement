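; Test player character for side-scrolling movement along X, using the ABP_Alucard animation blueprint and Enhanced Input actions alongside a legacy Forward axis.
; Jump, dash, down-slam and dash long jump are gated by state flags, built from launches, gravity and friction overrides, short timers and animation node jumps.
; Landing restores movement values and clears flags, with delays for some.
; Tick faces the controller along X velocity and prints an airborne tick count.
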(event Custom|JumpTime
  (if (Variables|Default|GetJumping)
    (bind _output_get (Variables|Default|SetJumpTimeVar (+ (Variables|Default|GetJumpTimeVar) 1.0)))
    (Development|PrintString (Utilities|String|ToString(Float) _output_get))))

(event Input|EnhancedActionEvents|EnhancedInputActionIA_Jump
  (params (ActionValue :type Boolean) (ElapsedSeconds :type Float%20%28double-precision%29) (TriggeredSeconds :type Float%20%28double-precision%29) (InputAction :type Input%20Action%20Object%20Reference :default "/Game/Controlls/InputActions/IA_Jump.IA_Jump"))
  (bind _charactermovement (Variables|Character|GetCharacterMovement))
  (:Triggered
    (if (not (Variables|Default|GetJumping)) :!label _label
      (if (Variables|Default|GetDownHold)
        (if (Variables|Default|GetDash)
          (if (not (Variables|Default|GetLongJump))
            (Variables|/Script/Engine.CharacterMovementComponent|SetGravityScale _charactermovement 1.0)
            (Variables|/Script/Engine.CharacterMovementComponent|SetFallingLateralFriction _charactermovement 0.0)
            (Character|LaunchCharacter (Math|Vector|MakeVector (* 0.0 (Variables|Default|GetRunPlayRate)) 0.0 5e+02) false false)
            (Variables|Default|SetLongJump true)
            (Variables|Default|SetJumping true)
            (Utilities|Time|SetTimerbyEvent (EventDispatchers|CreateEvent :!event EndAirDash) 0.05)))
        (else
          (Character|Jump)
          (Class|PaperZDAnimInstance|JumptoNode (Variables|Default|GetAnimInstance) "Airborne" "None")
          (Variables|Default|SetJumping true)
          (Variables|Default|SetDash false)))))
  (:Started
    (goto _label))
  (:Ongoing
    (Utilities|FlowControl|Delay 0.2)
    (goto _label))
  (:Canceled
    (Character|StopJumping :!label _label_2))
  (:Completed
    (goto _label_2)))

(event Input|EnhancedActionEvents|EnhancedInputActionIA_Down
  (params (ActionValue :type Boolean) (ElapsedSeconds :type Float%20%28double-precision%29) (TriggeredSeconds :type Float%20%28double-precision%29) (InputAction :type Input%20Action%20Object%20Reference :default "/Game/Controlls/InputActions/IA_Down.IA_Down"))
  (bind _charactermovement (Variables|Character|GetCharacterMovement))
  (:Triggered
    (Variables|Default|SetDownHold true :!label _label)
    (if (not (Variables|Default|GetSlam))
      (if (Variables|Default|GetJumping)
        (Variables|/Script/Engine.CharacterMovementComponent|SetMaxAcceleration _charactermovement 0.0)
        (Components|Movement|StopMovementImmediately _charactermovement)
        (Class|PaperZDAnimInstance|JumptoNode (Variables|Default|GetAnimInstance) "DDash_Jmp" "None")
        (Variables|/Script/Engine.CharacterMovementComponent|SetGravityScale (Variables|Character|GetCharacterMovement) 8e+03)
        (Variables|Default|SetSlam true))))
  (:Started
    (goto _label))
  (:Ongoing
    (goto _label))
  (:Canceled
    (Variables|Default|SetDownHold false :!label _label_2)
    (Class|PaperZDAnimInstance|JumptoNode (Variables|Default|GetAnimInstance) "Idle_Jmp" "None"))
  (:Completed
    (goto _label_2)))

(event Input|EnhancedActionEvents|EnhancedInputActionIA_Dash
  (params (ActionValue :type Boolean) (ElapsedSeconds :type Float%20%28double-precision%29) (TriggeredSeconds :type Float%20%28double-precision%29) (InputAction :type Input%20Action%20Object%20Reference :default "/Game/Controlls/InputActions/IA_Dash.IA_Dash"))
  (bind _charactermovement (Variables|Character|GetCharacterMovement))
  (:Triggered
    (if (not (Variables|Default|GetDash)) :!label _label
      (Components|Movement|StopMovementImmediately (Variables|Character|GetCharacterMovement))
      (Variables|/Script/Engine.CharacterMovementComponent|SetGravityScale _charactermovement 0.0)
      (Variables|/Script/Engine.CharacterMovementComponent|SetFallingLateralFriction _charactermovement 0.0)
      (Character|LaunchCharacter (Math|Vector|MakeVector (* (Variables|Default|GetLaunch%20Velocity%20X) (Variables|Default|GetRunPlayRate)) 0.0 0.0) false false)
      (Class|PaperZDAnimInstance|JumptoNode (Variables|Default|GetAnimInstance) "Airborne" "None")
      (Variables|Default|SetDash true)
      (Variables|Default|SetDownHold true)
      (Utilities|Time|SetTimerbyEvent (EventDispatchers|CreateEvent :!event EndAirDash) 0.05)))
  (:Started
    (goto _label))
  (:Canceled
    (Variables|Default|SetDownHold false :!label _label_2))
  (:Completed
    (goto _label_2)))

(event EventBeginPlay
  (Class|PaperZDAnimationComponent|SetAnimInstanceClass (Variables|Default|GetAnimationComponent) "/Game/Flipbook/Alucard/ABP_Alucard.ABP_Alucard_C")
  (bind _asplayer_controller (Utilities|Casting|CastToPlayerController (Pawn|GetController)))
  (Utilities|IsValid (PlayerController|LocalPlayerSubsystems|GetEnhancedInputLocalPlayerSubsystem _asplayer_controller)
    (:Is%20Valid
      (Input|AddMappingContext (PlayerController|LocalPlayerSubsystems|GetEnhancedInputLocalPlayerSubsystem _asplayer_controller) "/Game/Controlls/IM_Test.IM_Test" 0 "(bIgnoreAllPressedKeysUntilRelease=True,bForceImmediately=False,bNotifyUserSettings=False)"))))

(event EventOnWalkingOffLedge
  (params (PreviousFloorImpactNormal :type Vector%20%28by%20ref%29 :default "0, 0, 0") (PreviousFloorContactNormal :type Vector%20%28by%20ref%29 :default "0, 0, 0") (PreviousLocation :type Vector%20%28by%20ref%29 :default "0, 0, 0") (TimeDelta :type Float%20%28single-precision%29))
  (Class|PaperZDAnimInstance|JumptoNode (Variables|Default|GetAnimInstance) "Airborne" "None")
  (Variables|Default|SetJumping true))

(event EventTick
  (params (DeltaSeconds :type Float%20%28single-precision%29))
  (bind _returnvalue (Pawn|GetController))
  (bind _returnvalue_2 (Pawn|GetController))
  (|CallParentFunction DeltaSeconds)
  (CallFunction|JumpTime)
  (Math|Float|CompareFloat (.X (Math|Vector|BreakVector (Variables|/Script/Engine.MovementComponent|GetVelocity (Pawn|GetMovementComponent)))) 0.0
    (:>
      ;[0 0.4745 1] Look Right
      (Utilities|IsValid _returnvalue_2
        (:Is%20Valid
          (Pawn|SetControlRotation _returnvalue_2 (Math|Rotator|MakeRotator 0.0 0.0 0.0)))))
    (:<
      ;[0 0.4745 1] Look Left
      (Utilities|IsValid _returnvalue
        (:Is%20Valid
          (Pawn|SetControlRotation _returnvalue (Math|Rotator|MakeRotator 0.0 0.0 1.8e+02)))))))

(event EventOnLanded
  (params (Hit :type Hit%20Result%20Structure%20%28by%20ref%29))
  (Variables|Default|SetJumping false)
  (CallFunction|Reset)
  (Variables|Default|SetJumpTimeVar 0.0)
  (Utilities|FlowControl|Delay 0.1)
  (Variables|Default|SetSlam false)
  (Variables|Default|SetLongJump false)
  (Utilities|FlowControl|Delay 0.9)
  (Variables|Default|SetDash false))

(event Input|AxisEvents|InputAxisForward
  (params (AxisValue :type Float%20%28single-precision%29))
  (if (not (== AxisValue 0.0))
    (if (< AxisValue 0.0)
      (bind _output_get (Variables|Default|SetRunPlayRate -1.0))
      (Pawn|Input|AddMovementInput "5.000000,0.000000,0.000000" _output_get false)
      (else
        (bind _output_get_2 (Variables|Default|SetRunPlayRate 1.0))
        (Pawn|Input|AddMovementInput "5.000000,0.000000,0.000000" _output_get_2 false)))))

(fn ConstructionScript)

(fn EndAirDash
  (Variables|/Script/Engine.CharacterMovementComponent|SetGravityScale (Variables|Character|GetCharacterMovement) 1.0))

(fn Reset
  (bind _charactermovement (Variables|Character|GetCharacterMovement))
  (Variables|/Script/Engine.CharacterMovementComponent|SetGravityScale _charactermovement 1.0)
  (Variables|/Script/Engine.CharacterMovementComponent|SetMaxAcceleration _charactermovement 8e+04)
  (Variables|/Script/Engine.CharacterMovementComponent|SetFallingLateralFriction _charactermovement 213.382095)
  (Variables|/Script/Engine.CharacterMovementComponent|SetJumpZVelocity _charactermovement 6.5e+02))